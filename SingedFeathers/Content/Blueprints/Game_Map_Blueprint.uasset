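; Game map Blueprint that builds the map at BeginPlay as a grid of Paper2D tile map components.
; It loops from 1 to Width and 1 to Height, getting each cell's base tile and map location.
; A switch on TileId selects an AddPaperTileMapComponent call, placed at that location, with two IDs sharing one branch and a default for unlisted IDs.
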(event `self.ReceiveBeginPlay`
  (for _index (range 1 (+ (`self.width`) 1))
    (for _index_2 (range 1 (+ (`self.height`) 1))
      (bind _returnvalue (`self.GetBaseTile` _index _index_2))
      (bind _returnvalue_2 (`self.GetMapLocation` _index _index_2))
      (switch `int` (`Base_Tile.tileId` _returnvalue)
        (:`Default`
          (bind _returnvalue_3 (`KismetMathLibrary.Conv_VectorToTransform` _returnvalue_2))
          (`AddComponent|NODE_AddPaperTileMapComponent-5` :`self` _returnvalue :`RelativeTransform` _returnvalue_3))
        (:`0`
          (`AddComponent|NODE_AddPaperTileMapComponent-4` :`self` _returnvalue :`RelativeTransform` _returnvalue_3 :!label _label))
        (:`1`
          (goto _label))
        (:`3`
          (`AddComponent|NODE_AddPaperTileMapComponent-2` :`self` _returnvalue :`RelativeTransform` _returnvalue_3))
        (:`5`
          (`AddComponent|NODE_AddPaperTileMapComponent-3` :`self` _returnvalue :`RelativeTransform` _returnvalue_3))))))

(fn `UserConstructionScript`)